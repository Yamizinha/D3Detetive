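; Third statue in an ordered statue puzzle, which counts only when activated after the second statue.
; On Interact it plays a 2D sound and reads Valor2 from the Estatua02_BP found in the level.
; If that flag is true it sets its own Valor3; otherwise it clears the flags on Estatua01_BP and Estatua02_BP, resetting their progress.
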(event `/Game/inventorySistem/interact.interact`
  (params (player :type "Actor Object Reference"))
  (`GameplayStatics.PlaySound2D` (`self.Sound_3`) 1.0 1.0 0.0 null null)
  (bind _returnvalue (`GameplayStatics.GetActorOfClass` "/Game/Luiz/Puzzle_estatuas/BluePrints/Estatua02_BP.Estatua02_BP_C"))
  (if (`/Game/Luiz/Puzzle_estatuas/BluePrints/Estatua02_BP.Valor2` _returnvalue)
    (set `self.Valor3` true)
    (else
      (bind _returnvalue_2 (`GameplayStatics.GetActorOfClass` "/Game/Luiz/Puzzle_estatuas/BluePrints/Estatua01_BP.Estatua01_BP_C"))
      (set `/Game/Luiz/Puzzle_estatuas/BluePrints/Estatua01_BP.Valor1` false _returnvalue_2)
      (bind _returnvalue_3 (`GameplayStatics.GetActorOfClass` "/Game/Luiz/Puzzle_estatuas/BluePrints/Estatua02_BP.Estatua02_BP_C"))
      (set `/Game/Luiz/Puzzle_estatuas/BluePrints/Estatua02_BP.Valor2` false _returnvalue_3))))

(fn `UserConstructionScript`
  (`parent.UserConstructionScript`))