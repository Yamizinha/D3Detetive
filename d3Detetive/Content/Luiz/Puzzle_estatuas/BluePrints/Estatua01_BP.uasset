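; First statue of a statue puzzle, which sets its own Valor1 flag when the player interacts with it.
; Interact plays a sound, then looks up Estatua02_BP and Estatua03_BP by class and proceeds only if their Valor2 and Valor3 flags are both false.
; It then sets Valor1 true and writes false back to both other flags, which are already false at that point.
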(event `/Game/inventorySistem/interact.interact`
  (params (player :type "Actor Object Reference"))
  (`GameplayStatics.PlaySound2D` (`self.Sound_1`) 1.0 1.0 0.0 null null)
  (bind _returnvalue (`GameplayStatics.GetActorOfClass` "/Game/Luiz/Puzzle_estatuas/BluePrints/Estatua02_BP.Estatua02_BP_C"))
  (if (not (`/Game/Luiz/Puzzle_estatuas/BluePrints/Estatua02_BP.Valor2` _returnvalue))
    (bind _returnvalue_2 (`GameplayStatics.GetActorOfClass` "/Game/Luiz/Puzzle_estatuas/BluePrints/Estatua03_BP.Estatua03_BP_C"))
    (if (not (`/Game/Luiz/Puzzle_estatuas/BluePrints/Estatua03_BP.Valor3` _returnvalue_2))
      (set `self.Valor1` true)
      (`|ExecutionSequence`
        (:`then_0`
          (bind _returnvalue_3 (`GameplayStatics.GetActorOfClass` "/Game/Luiz/Puzzle_estatuas/BluePrints/Estatua02_BP.Estatua02_BP_C"))
          (set `/Game/Luiz/Puzzle_estatuas/BluePrints/Estatua02_BP.Valor2` false _returnvalue_3))
        (:`then_1`
          (bind _returnvalue_4 (`GameplayStatics.GetActorOfClass` "/Game/Luiz/Puzzle_estatuas/BluePrints/Estatua03_BP.Estatua03_BP_C"))
          (set `/Game/Luiz/Puzzle_estatuas/BluePrints/Estatua03_BP.Valor3` false _returnvalue_4))))))

(fn `UserConstructionScript`
  (`parent.UserConstructionScript`))