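; Candle number 5 in what appears to be a lights-out style puzzle, starting unlit with a timeline that flickers its point light intensity.
; InverterVela toggles its light, fire particle, shadow casting and EstadoVela5, then flips neighbouring candles 4 and 6, found by GetActorOfClass.
; NoLoopVela5 toggles only this candle, so flips requested from outside do not cascade.
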(event `self.ReceiveBeginPlay`
  ;[1 1 1] Efeitos visuais da vela ficando mais forte efraca
  (`|ExecutionSequence`
    (:`then_0`
      (bind (_direction _intensidade) (`Timeline|VelaTimeline`)
        (:`Update`
          (`LightComponent.SetIntensity` (`self.PointLight`) (`KismetMathLibrary.Lerp` (`self.MinIntensity`) (`self.MaxIntensity`) _intensidade)))))
    (:`then_1`
      (bind _output_get (set `self.X` false :!label _label))
      ;[1 1 1] Desativa a luz e a particula do fogo para o player
      (`SceneComponent.SetVisibility` (`self.PointLight`) _output_get false)
      (`SceneComponent.SetVisibility` (`self.ParticleSystem`) _output_get false)
      (`PrimitiveComponent.SetCastShadow` (`self.Vela`) (not _output_get))
      (set `self.EstadoVela5` (`self.Apagada`)))))

(event `InverterVela`
  (if (`self.EstadoVela5`)
    (bind _output_get (set `self.X` false))
    ;[1 1 1] Desativa a luz e a particula do fogo para o player
    (`SceneComponent.SetVisibility` (`self.PointLight`) _output_get false)
    (`SceneComponent.SetVisibility` (`self.ParticleSystem`) _output_get false)
    (`PrimitiveComponent.SetCastShadow` (`self.Vela`) (not _output_get))
    (set `self.EstadoVela5` (`self.Apagada`))
    (else
      (bind _output_get_2 (set `self.X` false))
      ;[1 1 1] Ativa Luz e a Particula do fogo para o player
      (`SceneComponent.SetVisibility` (`self.PointLight`) (not _output_get_2) false)
      (`SceneComponent.SetVisibility` (`self.ParticleSystem`) (not _output_get_2) false)
      (`PrimitiveComponent.SetCastShadow` (`self.Vela`) _output_get_2)
      (set `self.EstadoVela5` (`self.Acesa`))))
  ;[1 1 1] Inverte As velas ao lado
  (bind _returnvalue (`GameplayStatics.GetActorOfClass` "/Game/Miranda/Velas/BP_Vela4.BP_Vela4_C"))
  (`/Game/Miranda/Velas/BP_Vela4.NoLoopVela4` _returnvalue)
  (bind _returnvalue_2 (`GameplayStatics.GetActorOfClass` "/Game/Miranda/Velas/BP_VelaMagraGrande6.BP_VelaMagraGrande6_C"))
  (`/Game/Miranda/Velas/BP_VelaMagraGrande6.NoLoopVela6` _returnvalue_2))

(event `NoLoopVela5`
  (if (`self.EstadoVela5`)
    (goto _label)
    (else
      (bind _output_get (set `self.X` false))
      ;[1 1 1] Ativa Luz e a Particula do fogo para o player
      (`SceneComponent.SetVisibility` (`self.PointLight`) (not _output_get) false)
      (`SceneComponent.SetVisibility` (`self.ParticleSystem`) (not _output_get) false)
      (`PrimitiveComponent.SetCastShadow` (`self.Vela`) _output_get)
      (set `self.EstadoVela5` (`self.Acesa`)))))

(fn `UserConstructionScript`)