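; BP_VelaMagraGrande3 is an interactable candle, apparently one of a linked toggle puzzle, with a timeline-driven flickering light.
; Interact uses a FlipFlop to switch light, fire particles, shadow casting and EstadoVela3, then toggles neighboring BP_VelaGordaGrand2 and BP_Vela4 candles.
; NoLoopVela3 toggles only this candle without propagating, branching on EstadoVela3 rather than sharing the FlipFlop's state.
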(event `self.ReceiveBeginPlay`
  ;[1 1 1] Efeitos visuais da vela ficando mais forte efraca
  (bind (_direction _intensidade) (`Timeline|VelaTimeline`)
    (:`Update`
      (`LightComponent.SetIntensity` (`self.PointLight`) (`KismetMathLibrary.Lerp` (`self.MinIntensity`) (`self.MaxIntensity`) _intensidade)))))

(event `InverterVela`)

(event `/Game/inventorySistem/interact.interact`
  (params (player :type "Actor Object Reference"))
  (`/Engine/EditorBlueprintResources/StandardMacros.FlipFlop`
    (:`A`
      (bind _output_get (set `self.X` false))
      ;[1 1 1] Desativa a luz e a particula do fogo para o player
      (`SceneComponent.SetVisibility` (`self.PointLight`) _output_get false)
      (`SceneComponent.SetVisibility` (`self.ParticleSystem`) _output_get false)
      (`PrimitiveComponent.SetCastShadow` (`self.Vela`) (not _output_get))
      (set `self.EstadoVela3` (`self.Apagada`)))
    (:`B`
      (bind _output_get_2 (set `self.X` false))
      ;[1 1 1] Ativa Luz e a Particula do fogo para o player
      (`SceneComponent.SetVisibility` (`self.PointLight`) (not _output_get_2) false)
      (`SceneComponent.SetVisibility` (`self.ParticleSystem`) (not _output_get_2) false)
      (`PrimitiveComponent.SetCastShadow` (`self.Vela`) _output_get_2)
      (set `self.EstadoVela3` (`self.Acesa`))))
  ;[1 1 1] Inverte As velas ao lado
  (bind _outactors (`GameplayStatics.GetAllActorsOfClass` "/Game/Miranda/Velas/BP_VelaGordaGrand2.BP_VelaGordaGrand2_C"))
  (`/Game/Miranda/Velas/BP_VelaGordaGrand2.NoLoopVela2` _outactors)
  (bind _outactors_2 (`GameplayStatics.GetAllActorsOfClass` "/Game/Miranda/Velas/BP_Vela4.BP_Vela4_C"))
  (`/Game/Miranda/Velas/BP_Vela4.NoLoopVela4` _outactors_2))

(event `NoLoopVela3`
  (if (`self.EstadoVela3`)
    (bind _output_get (set `self.X` false))
    ;[1 1 1] Desativa a luz e a particula do fogo para o player
    (`SceneComponent.SetVisibility` (`self.PointLight`) _output_get false)
    (`SceneComponent.SetVisibility` (`self.ParticleSystem`) _output_get false)
    (`PrimitiveComponent.SetCastShadow` (`self.Vela`) (not _output_get))
    (set `self.EstadoVela3` (`self.Apagada`))
    (else
      (bind _output_get_2 (set `self.X` false))
      ;[1 1 1] Ativa Luz e a Particula do fogo para o player
      (`SceneComponent.SetVisibility` (`self.PointLight`) (not _output_get_2) false)
      (`SceneComponent.SetVisibility` (`self.ParticleSystem`) (not _output_get_2) false)
      (`PrimitiveComponent.SetCastShadow` (`self.Vela`) _output_get_2)
      (set `self.EstadoVela3` (`self.Acesa`)))))

(fn `UserConstructionScript`)