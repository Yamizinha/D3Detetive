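; BP_Vela is a candle with a point light and flame particle that can be lit or put out.
; Its construction script calls SetAcesa to match light, flame and mesh shadow to the Acesa flag, with shadows cast only when unlit.
; On BeginPlay, a timeline varies the light intensity between minimum and maximum.
; InverterVela alternates off and on through a FlipFlop, always extinguishing first and using a separate Apagada flag to relight.
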(event `self.ReceiveBeginPlay`
  (bind (_direction _intensidade) (`Timeline|VelaTimeline`)
    (:`Update`
      (`LightComponent.SetIntensity` (`self.PointLight`) (`KismetMathLibrary.Lerp` (`self.MinIntensity`) (`self.MaxIntensity`) _intensidade)))))

(event `InverterVela`
  (`/Engine/EditorBlueprintResources/StandardMacros.FlipFlop`
    (:`A`
      (bind _output_get (set `self.Acesa` false))
      ;[1 1 1] Desativa a luz e a particula do fogo para o player
      (`SceneComponent.SetVisibility` (`self.PointLight`) _output_get false)
      (`SceneComponent.SetVisibility` (`self.ParticleSystem`) _output_get false)
      (`PrimitiveComponent.SetCastShadow` (`self.Vela`) (not _output_get))
      (`KismetSystemLibrary.PrintString` "Apaga"))
    (:`B`
      (bind _output_get_2 (set `self.Apagada` false))
      ;[1 1 1] Ativa Luz e a Particula do fogo para o player
      (`SceneComponent.SetVisibility` (`self.PointLight`) (not _output_get_2) false)
      (`SceneComponent.SetVisibility` (`self.ParticleSystem`) (not _output_get_2) false)
      (`PrimitiveComponent.SetCastShadow` (`self.Vela`) _output_get_2)
      (`KismetSystemLibrary.PrintString` "Acende"))))

(fn `SetAcesa`
  (params (Acesa :type Boolean :default false))
  (bind _output_get (set `self.Acesa` Acesa))
  ;[1 1 1] Desativa a luz e a particula do fogo para o player
  (`SceneComponent.SetVisibility` (`self.PointLight`) _output_get false)
  (`SceneComponent.SetVisibility` (`self.ParticleSystem`) _output_get false)
  (`PrimitiveComponent.SetCastShadow` (`self.Vela`) (not _output_get)))

(fn `UserConstructionScript`
  (`self.SetAcesa` (`self.Acesa`)))