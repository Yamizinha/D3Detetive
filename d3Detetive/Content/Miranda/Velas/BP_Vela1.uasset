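; BP_Vela1 is a toggleable candle that appears to be part of a linked-candle puzzle, with light intensity animated by a timeline.
; InverterVela alternates via FlipFlop between lit and unlit, setting flame, light, shadow casting and EstadoVela1, then toggles neighbor BP_VelaGordaGrand2, found by class.
; NoLoopVela1 toggles this candle from EstadoVela1 without propagating, preventing infinite loops.
; The FlipFlop ignores EstadoVela1, so the two toggle paths track state independently.
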(event `self.ReceiveBeginPlay`
  ;[1 1 1] Efeitos visuais da vela ficando mais forte efraca
  (bind (_direction _intensidade) (`Timeline|VelaTimeline`)
    (:`Update`
      (`LightComponent.SetIntensity` (`self.PointLight`) (`KismetMathLibrary.Lerp` (`self.MinIntensity`) (`self.MaxIntensity`) _intensidade)))))

(event `InverterVela`
  (`/Engine/EditorBlueprintResources/StandardMacros.FlipFlop`
    (:`A`
      (bind _output_get (set `self.X` false))
      ;[1 1 1] Desativa a luz e a particula do fogo para o player
      (`SceneComponent.SetVisibility` (`self.PointLight`) _output_get false)
      (`SceneComponent.SetVisibility` (`self.ParticleSystem`) _output_get false)
      (`PrimitiveComponent.SetCastShadow` (`self.Vela`) (not _output_get))
      (set `self.EstadoVela1` (`self.Apagada`)))
    (:`B`
      (bind _output_get_2 (set `self.X` false))
      ;[1 1 1] Ativa Luz e a Particula do fogo para o player
      (`SceneComponent.SetVisibility` (`self.PointLight`) (not _output_get_2) false)
      (`SceneComponent.SetVisibility` (`self.ParticleSystem`) (not _output_get_2) false)
      (`PrimitiveComponent.SetCastShadow` (`self.Vela`) _output_get_2)
      (set `self.EstadoVela1` (`self.Acesa`))))
  ;[1 1 1] Inverte As velas ao lado
  (bind _returnvalue (`GameplayStatics.GetActorOfClass` "/Game/Miranda/Velas/BP_VelaGordaGrand2.BP_VelaGordaGrand2_C"))
  (`/Game/Miranda/Velas/BP_VelaGordaGrand2.NoLoopVela2` _returnvalue))

(event `NoLoopVela1`
  ;[1 1 1] Previne Loop Infinito
  (if (`self.EstadoVela1`)
    (bind _output_get (set `self.X` false))
    ;;[1 1 1] Desativa a luz e a particula do fogo para o player
    (`SceneComponent.SetVisibility` (`self.PointLight`) _output_get false)
    (`SceneComponent.SetVisibility` (`self.ParticleSystem`) _output_get false)
    (`PrimitiveComponent.SetCastShadow` (`self.Vela`) (not _output_get))
    (set `self.EstadoVela1` (`self.Apagada`))
    (else
      (bind _output_get_2 (set `self.X` false))
      ;;[1 1 1] Ativa Luz e a Particula do fogo para o player
      (`SceneComponent.SetVisibility` (`self.PointLight`) (not _output_get_2) false)
      (`SceneComponent.SetVisibility` (`self.ParticleSystem`) (not _output_get_2) false)
      (`PrimitiveComponent.SetCastShadow` (`self.Vela`) _output_get_2)
      (set `self.EstadoVela1` (`self.Acesa`)))))

(fn `UserConstructionScript`)